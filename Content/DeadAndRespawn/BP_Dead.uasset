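; BP_Dead is a death trigger that plays a death scene and respawns the player when a BP_ThirdPersonCharacter overlaps it.
; On overlap, it opens the DeadScene source on the DeadVideo media player and shows a WB_DeadScene widget.
; After a fixed delay meant to match the video length, it removes the widget and moves the character to Respawn.
; Respawn's location is relative to the actor, while its rotation is applied untransformed.
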(event `self.Trigger.OnComponentBeginOverlap`
  (params (OverlappedComponent :type "PrimitiveComponent Object Reference") (OtherActor :type "Actor Object Reference") (OtherComp :type "PrimitiveComponent Object Reference") (OtherBodyIndex :type Integer) (bFromSweep :type Boolean) (SweepResult :type "HitResult Structure (by ref)"))
  (bind (_respawn_location _respawn_rotation) (`KismetMathLibrary.BreakTransform` (`self.Respawn`)))
  (bind _asbp_third_person_character (cast `/Game/ThirdPerson/Blueprints/BP_ThirdPersonCharacter` OtherActor))
  ;[1 1 1] DeadScene(Delay長度=影片長度)
  (`MediaPlayer.OpenSource` (`self.DeadVideo`) "/Game/DeadAndRespawn/DeadScene.DeadScene")
  (bind _returnvalue (`|CreateWidget` "/Game/DeadAndRespawn/WB_DeadScene.WB_DeadScene_C"))
  (`UserWidget.AddToViewport` _returnvalue 0)
  (`KismetSystemLibrary.Delay` 2.0)
  (`Widget.RemoveFromParent` _returnvalue)
  (`self.K2_SetActorLocationAndRotation` _asbp_third_person_character (`KismetMathLibrary.TransformLocation` (`self.GetTransform`) _respawn_location) _respawn_rotation false false))

(fn `UserConstructionScript`)