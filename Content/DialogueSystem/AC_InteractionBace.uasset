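; AC_InteractionBace is an interaction base in the dialogue system that exposes shared hit-tracking state.
; Getters return the current and previous hit actors, each paired with a validity flag.
; A RecheckHit flag is read and toggled through its own getter and enable/disable functions.
; It contains no tracing or active event logic, and nothing here assigns the hit actors.
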(fn `DisableHitRecheck`
  (set `self.bRecheckHit?` false))

(fn `EnableHitRecheck`
  (set `self.bRecheckHit?` true))

(fn `GetCurrentHit`
  (returns (ReturnValue :type Boolean) (CurrentHitActor :type "Actor Object Reference"))
  (bind _currenthitactor (`self.CurrentHitActor`))
  (return (`KismetSystemLibrary.IsValid` _currenthitactor) _currenthitactor))

(fn `GetPreviousHit`
  (returns (ReturnValue :type Boolean) (PrevHitActor :type "Actor Object Reference"))
  (bind _prevhitactor (`self.PrevHitActor`))
  (return (`KismetSystemLibrary.IsValid` _prevhitactor) _prevhitactor))

(fn `GetRecheckHit`
  (returns (`bRecheckHit?` :type Boolean))
  (return (`self.bRecheckHit?`)))