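; AC_Interaction is an interaction component in the dialogue system that updates highlighting and interact input for the actor the player targets.
; On a hit it outlines the current actor, clears the previous one's outline and adds the IMC_Interact mapping through the controller's AC_InputControls component.
; Without a hit it clears the previous outline and removes the mapping.
; TriggerInteract extends the parent implementation, then removes the mapping.
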(fn `TriggerInteract`
  (`parent.TriggerInteract`)
  (`/Game/DialogueSystem/AC_InputControls.RemoveInputMapping` (`Actor.GetComponentByClass` (`GameplayStatics.GetPlayerController` 0) "/Game/DialogueSystem/AC_InputControls.AC_InputControls_C") "/Game/ThirdPerson/Input/IMC_Interact.IMC_Interact"))

(fn `UpdateInteractState`
  (params (`bHit?` :type Boolean))
  (if `bHit?`
    (message `/Game/DialogueSystem/BPI_Interact.SetOutlineState` (`self.CurrentHitActor`) true)
    (`/Engine/EditorBlueprintResources/StandardMacros.IsValid` (`self.PrevHitActor`)
      (:`Is Valid`
        (message `/Game/DialogueSystem/BPI_Interact.SetOutlineState` (`self.PrevHitActor`) false))
      (:`Is Not Valid`
        _))
    (`/Game/DialogueSystem/AC_InputControls.AddInputMapping` (`Actor.GetComponentByClass` (`GameplayStatics.GetPlayerController` 0) "/Game/DialogueSystem/AC_InputControls.AC_InputControls_C") "/Game/ThirdPerson/Input/IMC_Interact.IMC_Interact")
    (else
      (`/Engine/EditorBlueprintResources/StandardMacros.IsValid` (`self.PrevHitActor`)
        (:`Is Valid`
          (message `/Game/DialogueSystem/BPI_Interact.SetOutlineState` (`self.PrevHitActor`) false))
        (:`Is Not Valid`
          _))
      (`/Game/DialogueSystem/AC_InputControls.RemoveInputMapping` (`Actor.GetComponentByClass` (`GameplayStatics.GetPlayerController` 0) "/Game/DialogueSystem/AC_InputControls.AC_InputControls_C") "/Game/ThirdPerson/Input/IMC_Interact.IMC_Interact"))))