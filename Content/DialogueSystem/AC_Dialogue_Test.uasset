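; Test dialogue component for the NPC TheTestGuy, a commented example of branching conversation built on a parent dialogue class.
; The Dialogue override switches on DialogueTreeIndex, chaining AddDialogue nodes that branch on the chosen option once their State is Pass Through.
; Tree 0 is a math quiz whose endings advance to tree 1, rewind progress or clear it before closing the conversation.
; Tree 1 gives a random closing line.
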(fn `Dialogue`
  (`parent.Dialogue`)
  (switch `int` (`self.DialogueTreeIndex`)
    (:`0`
      ;[1 1 1] 問題(藍)跟選項(綠)
      (bind (_state _optionindex) (`self.AddDialogue` "TheTestGuy" "請問1+1=?" (`|MakeArray` "2" "5" :!type "Text")))
      (switch `/Game/DialogueSystem/Enum_DialogueState` _state
        (:`NewEnumerator0`
          ;[1 1 1] 前面幾個選項就放多少pin
          (switch `int` _optionindex
            (:`0`
              (bind (_state_2 _optionindex_2) (`self.AddDialogue` "TheTestGuy" "基礎數學哈哈" (`|MakeArray` "那你問屁" "謝謝" :!type "Text")))
              (switch `/Game/DialogueSystem/Enum_DialogueState` _state_2
                (:`NewEnumerator0`
                  (switch `int` _optionindex_2
                    (:`0`
                      (bind _state_3 (`self.AddDialogue` "TheTestGuy" "好玩嘛:)" (`|MakeArray` "謝囉" :!type "Text")))
                      (switch `/Game/DialogueSystem/Enum_DialogueState` _state_3
                        (:`NewEnumerator0`
                          ;[1 1 1] 對話結束 回到第一個switch on int的多少就輸多少
                          (`self.SetDialogueTreeIndex` 1)
                          (`self.CloseConversation`))))
                    (:`1`
                      (bind _state_4 (`self.AddDialogue` "TheTestGuy" "真有禮貌 好孩子" (`|MakeArray` "不會" :!type "Text")))
                      (switch `/Game/DialogueSystem/Enum_DialogueState` _state_4
                        (:`NewEnumerator0`
                          ;[1 1 1] 回到前第x個add dialogue就輸x-1
                          (`self.RemoveDialogueProgress` 2)
                          (`self.CloseConversation`))))))))
            (:`1`
              (bind _state_5 (`self.AddDialogue` "TheTestGuy" "不是 哥們 這麼簡單都可以答錯嗎" (`|MakeArray` "乾你屁事" "我頭腦不好" :!type "Text")))
              (switch `/Game/DialogueSystem/Enum_DialogueState` _state_5
                (:`NewEnumerator0`
                  ;[1 1 1] 結束對話
                  (`self.ClearDialogueProgress`)
                  (`self.CloseConversation`))))))))
    (:`1`
      (bind _state_6 (`self.AddDialogue` "TheTestGuy" (select `int` (`KismetMathLibrary.RandomIntegerInRange` 0 1) :`0` "測試結束~" :`1` "大成功好欸" :!type "Text") (`|MakeArray` "掰" :!type "Text")))
      (switch `/Game/DialogueSystem/Enum_DialogueState` _state_6
        (:`NewEnumerator0`
          (`self.ClearDialogueProgress`)
          (`self.CloseConversation`))))))