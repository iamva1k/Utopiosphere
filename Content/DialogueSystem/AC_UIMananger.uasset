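; Actor component that manages the on-screen interaction prompt for the player's interaction system.
; On BeginPlay it caches the player character's AC_InteractionBace component, then every Tick checks its current hit.
; While something is hit, it creates a WB_InteractionPrompt once with the hit actor's text and feeds it hold progress as a normalized ratio.
; When the hit is lost, it removes and clears the widget.
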(event `self.ReceiveBeginPlay`
  (set `self.InteractionComponent` (`Actor.GetComponentByClass` (`GameplayStatics.GetPlayerCharacter` 0) "/Game/DialogueSystem/AC_InteractionBace.AC_InteractionBace_C")))

(event `self.ReceiveTick`
  (params (DeltaSeconds :type "Float (single-precision)"))
  (`self.ShowInteractPrompt`))

(fn `ShowInteractPrompt`
  (bind _interactioncomponent (`self.InteractionComponent`))
  (bind (_returnvalue _currenthitactor) (`/Game/DialogueSystem/AC_InteractionBace.GetCurrentHit` (`self.InteractionComponent`)))
  (if _returnvalue
    (`/Engine/EditorBlueprintResources/StandardMacros.IsValid` (`self.InteractPrompt`)
      (:`Is Valid`
        _)
      (:`Is Not Valid`
        (bind _interacttext (message `/Game/DialogueSystem/BPI_Interact.GetInteractText` _currenthitactor))
        (bind _returnvalue_2 (`|CreateWidget` "/Game/DialogueSystem/WB_InteractionPrompt.WB_InteractionPrompt_C" null _interacttext))
        (bind _output_get (set `self.InteractPrompt` _returnvalue_2))
        (`UserWidget.AddToViewport` _output_get 3)))
    (`/Game/DialogueSystem/WB_InteractionPrompt.UpdateTimer` (`self.InteractPrompt`) (/ (`/Game/DialogueSystem/AC_InteractionBace.CurrentHoldDuration` _interactioncomponent) (`/Game/DialogueSystem/AC_InteractionBace.InteractHoldTimer` _interactioncomponent)))
    (else
      (`/Engine/EditorBlueprintResources/StandardMacros.IsValid` (`self.InteractPrompt`)
        (:`Is Valid`
          (`Widget.RemoveFromParent` (`self.InteractPrompt`))
          (set `self.InteractPrompt` null))))))