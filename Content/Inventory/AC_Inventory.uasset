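; Inventory component that lets its connected actor pick up items and store them in a name-keyed map.
; On completed pickup input, a camera-forward sphere trace with debug drawing passes the hit actor to TryAddItem.
; TryAddItem reads item data from AC_MasterPickUpItem actors, adds new names and prints a confirmation.
; Duplicates go to IncreaseItemAmount, whose increment logic is disconnected, so their stored amount never changes despite the "Added" message.
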(event `EnhancedInput|/Game/ThirdPerson/Input/Actions/IA_PickUp`
  (params (ActionValue :type Boolean) (ElapsedSeconds :type "Float (double-precision)") (TriggeredSeconds :type "Float (double-precision)") (InputAction :type "InputAction Object Reference" :default "/Game/ThirdPerson/Input/Actions/IA_PickUp.IA_PickUp"))
  (bind _connectedactor (`self.ConnectedActor`))
  (bind _followcamera (`/Game/ThirdPerson/Blueprints/BP_ThirdPersonCharacter.FollowCamera` _connectedactor))
  (bind _returnvalue (`SceneComponent.K2_GetComponentLocation` _followcamera))
  (:`Completed`
    (bind (_outhit _returnvalue_2) (`KismetSystemLibrary.SphereTraceSingle` :`Start` _returnvalue :`End` (+ _returnvalue (* (`SceneComponent.GetForwardVector` _followcamera) (+ (`SpringArmComponent.TargetArmLength` (`/Game/ThirdPerson/Blueprints/BP_ThirdPersonCharacter.CameraBoom` _connectedactor)) 300.0))) :`Radius` 10.0 :`TraceChannel` "TraceTypeQuery1" :`DrawDebugType` "ForDuration"))
    (if _returnvalue_2
      (`self.TryAddItem` (`.HitActor` (`GameplayStatics.BreakHitResult` _outhit))))))

(fn `AddItemToInventory`
  (params (Item :type "/Game/Inventory/S_ItemData Structure"))
  (`BlueprintMapLibrary.Map_Add` (`self.Inventory`) (`.Name_3_290AB9F84F4E6225B8448996AF00E883` (break `/Game/Inventory/S_ItemData` Item)) Item))

(fn `IncreaseItemAmount`
  (params (Item :type "/Game/Inventory/S_ItemData Structure"))
  (locals (ItemName :type String)))

(fn `IsItemAlreadyInInventory`
  (params (Item :type "/Game/Inventory/S_ItemData Structure"))
  (returns (ReturnValue :type Boolean))
  (return (`BlueprintMapLibrary.Map_Contains` (`self.Inventory`) (`.Name_3_290AB9F84F4E6225B8448996AF00E883` (break `/Game/Inventory/S_ItemData` Item)))))

(fn `TryAddItem`
  (params (HitActor :type "Actor Object Reference"))
  (returns (`Added?` :type Boolean))
  (locals (CurrentItem :type "/Game/Inventory/S_ItemData Structure"))
  (bind _currentitem (`local.CurrentItem`))
  (bind _asac_master_pick_up_item (cast `/Game/Inventory/AC_MasterPickUpItem` HitActor)
    (:`then`
      (bind _output_get (set `local.CurrentItem` (`/Game/Inventory/AC_MasterPickUpItem.GetItemData` _asac_master_pick_up_item)))
      (if (`self.IsItemAlreadyInInventory` _output_get)
        (`self.IncreaseItemAmount` (`local.CurrentItem`))
        (else
          (`self.AddItemToInventory` _currentitem)))
      (`KismetSystemLibrary.PrintString` (`KismetStringLibrary.Concat_StrStr` (`.Name_3_290AB9F84F4E6225B8448996AF00E883` (break `/Game/Inventory/S_ItemData` _currentitem)) "Added"))
      (return true))
    (:`CastFailed`
      (set `local.CurrentItem` (struct))
      (return false))))